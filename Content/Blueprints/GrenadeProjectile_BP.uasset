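; Grenade projectile actor that plays a launcher sound on spawn and explodes on hit or after a short fuse delay.
; Both triggers feed an Explode event that spawns particle and sound effects, applies radial damage credited to the instigator, and destroys the actor.
; A debug sphere showing the damage radius is drawn after the destroy call.
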(event Custom|Explode
  (bind _returnvalue (Transformation|GetActorLocation))
  (Effects|SpawnEmitteratLocation "/Game/WeaponEffects/Explosion/P_Explosion.P_Explosion" _returnvalue)
  (Audio|SpawnSoundatLocation "/Game/WeaponSounds/Grenade_Explosion.Grenade_Explosion" _returnvalue "0, 0, 0" 1.0 1.0 0.0 0 0)
  (Game|Damage|ApplyRadialDamage 1e+02 _returnvalue (Variables|Default|GetDamageRadius) 0 0 self (Game|GetInstigatorController) false "ECC_Visibility")
  (Actor|DestroyActor)
  (Rendering|Debug|DrawDebugSphere _returnvalue (Variables|Default|GetDamageRadius) 12 "(R=1.000000,G=0.000000,B=0.049486,A=1.000000)" 1.0 2.0))

(event EventBeginPlay
  (Audio|SpawnSoundatLocation "/Game/WeaponSounds/Grenade_Launcher.Grenade_Launcher" (Transformation|GetActorLocation) "0, 0, 0" 1.0 1.0 0.0 0 0)
  (Utilities|FlowControl|Delay 1.0)
  (CallFunction|Explode))

(event Collision|EventHit
  (params (MyComp :type Primitive%20Component%20Object%20Reference) (Other :type Actor%20Object%20Reference) (OtherComp :type Primitive%20Component%20Object%20Reference) (bSelfMoved :type Boolean) (HitLocation :type Vector :default "0, 0, 0") (HitNormal :type Vector :default "0, 0, 0") (NormalImpulse :type Vector :default "0, 0, 0") (Hit :type Hit%20Result%20Structure%20%28by%20ref%29))
  (CallFunction|Explode))

(fn ConstructionScript)